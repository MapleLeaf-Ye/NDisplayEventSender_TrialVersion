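; Example actor demonstrating a plugin that distributes Blueprint events and functions across nDisplay cluster nodes.
; It contrasts manual JSON cluster events with TransformNDisFunc, which leads an event or function so the following logic runs on every node.
; Test cases cover parameter types and the older TriggleMultiNodeEventSimple node, which separates all-node and primary-only logic.
; Deliberate misuse examples show misplaced transform nodes, nested converted calls and rapid repeat calls from Tick.
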(event `MyEvent`
  (params (printedString :type String) (addInt :type Integer))
  ;[0 1 0.9935] 插件能做什么？  What do plug-ins do?
  ;;[0.963 1 0.4316] 希望分发到各个节点的逻辑   The logic that you want to distribute to each node
  (`KismetSystemLibrary.PrintString` printedString)
  (set `self.TestInt` (+ addInt 1)))

(event `self.ReceiveBeginPlay`
  ;[0 1 0.9935] 插件能做什么？  What do plug-ins do?
  ;;[0.0142 0 1] 原始实现方法  Original implementation method
  (`DisplayClusterBlueprintAPI.AddClusterEventListener` (`DisplayClusterBlueprintLib.GetAPI`) self))

(event `self.OnClusterEventJson`
  (params (Event :type "DisplayClusterClusterEventJson Structure (by ref)"))
  (bind ((`Name` _name) (`Parameters` _parameters)) (break `DisplayClusterClusterEventJson` Event))
  ;[0 1 0.9935] 插件能做什么？  What do plug-ins do?
  ;;[0.0142 0 1] 原始实现方法  Original implementation method
  (switch `string` _name
    (:`MyEvent`
      (`self.MyEvent` (`BlueprintMapLibrary.Map_Find` _parameters "printedString") (`KismetStringLibrary.Conv_StringToInt` (`BlueprintMapLibrary.Map_Find` _parameters "addInt"))))))

(event `NewExecuteMyEvent`
  (params (printedString :type String) (addInt :type Integer))
  ;[0 1 0.9935] 插件能做什么？  What do plug-ins do?
  ;;[1 0 0.04992] 插件实现方法   Plugin implementation method
  (`|TransformNDisFunc` printedString addInt)
  (`self.MyEvent` printedString addInt))

(event `ExecuteMyEvent`
  (params (printedString :type String) (addInt :type Integer))
  ;[0 1 0.9935] 插件能做什么？  What do plug-ins do?
  ;;[0.0142 0 1] 原始实现方法  Original implementation method
  (`DisplayClusterBlueprintAPI.EmitClusterEventJson` (`DisplayClusterBlueprintLib.GetAPI`) (make `DisplayClusterClusterEventJson` :`Name` "MyEvent" :`Parameters` (`|MakeMap` "printedString" printedString "addInt" (`KismetStringLibrary.Conv_IntToString` addInt))) false))

(event `NewMyEvent`
  (params (printedString :type String) (addInt :type Integer))
  ;[0 1 0.9935] 插件能做什么？  What do plug-ins do?
  ;;[1 0 0.04992] 形式二   The Second form
  (`|TransformNDisFunc` printedString addInt)
  (`KismetSystemLibrary.PrintString` printedString)
  (set `self.TestInt` (+ addInt 1)))

(event `TestEvent1`
  ;[1 1 1] 用于多节点事件分发，只需要为其指定函数的参数，就可以在主节点上将事件分发并执行在各个结点上，注意这个节点必须被放置在自定义事件或者函数的第一个
  ; 支持函数和事件的转换，但尽量保证转换节点放置在第一个，否则转换节点前面的逻辑可能会被执行多次
  ; 注意：
  ;  1.可以使用普通函数或者事件去调用被转换后的函数或事件，且可以连续调用，但是不要短时间内调用同一个被转换后的函数或者事件（名字相同的）多次，否则可能只能执行一次
  ;  2.正在转换的函数或者事件内部请不要去调用其他已转换的事件或者函数，否则可能会导致执行顺序混乱且多次执行
  ;  3.转换事件尽量写在每个节点都会存在的对象上（因为转换节点需要通过该对象寻找函数，如果写在一个非各个结点都存在的对象上会导致那个节点无法执行目标函数）
  ;  4.尽量只用ExecuteMultiNodeEvent_Auto节点，如果非要使用ExecuteMultiNodeEvent那么每个节点需要执行的逻辑请写在NormalExe引脚，如果需要主机特例执行逻辑则写在MultiNodeExe（因为该引脚是主机分发事件执行前执行的，其它节点不执行该引脚的逻辑）
  ;  5.转换函数或事件的参数顺序必须一对一，例如：函数参数一必须对应转换节点参数一，函数参数二必须对应转换节点参数二
  ;  6.定义的函数请不要有返回值，如果实在需要返回值可以实现逻辑内结果保存到一个中间类，各个结点再去取
  ;  7.转换过后的函数或事件在非Ndisplay启动模式下也同样可以当普通函数执行，不受任何影响
  (`|TransformNDisFunc`)
  ;;[1 1 1] 分发节点后面的逻辑就会执行在各个节点上（The logic behind the distribution node is executed on each node）
  (`KismetSystemLibrary.PrintString` "TODO") ; TODO，这边的逻辑就会执行在各个节点上
)

(event `ERROR_TestEvent1`
  ;[1 1 1] 用于多节点事件分发，只需要为其指定函数的参数，就可以在主节点上将事件分发并执行在各个结点上，注意这个节点必须被放置在自定义事件或者函数的第一个
  ; 支持函数和事件的转换，但尽量保证转换节点放置在第一个，否则转换节点前面的逻辑可能会被执行多次
  ; 注意：
  ;  1.可以使用普通函数或者事件去调用被转换后的函数或事件，且可以连续调用，但是不要短时间内调用同一个被转换后的函数或者事件（名字相同的）多次，否则可能只能执行一次
  ;  2.正在转换的函数或者事件内部请不要去调用其他已转换的事件或者函数，否则可能会导致执行顺序混乱且多次执行
  ;  3.转换事件尽量写在每个节点都会存在的对象上（因为转换节点需要通过该对象寻找函数，如果写在一个非各个结点都存在的对象上会导致那个节点无法执行目标函数）
  ;  4.尽量只用ExecuteMultiNodeEvent_Auto节点，如果非要使用ExecuteMultiNodeEvent那么每个节点需要执行的逻辑请写在NormalExe引脚，如果需要主机特例执行逻辑则写在MultiNodeExe（因为该引脚是主机分发事件执行前执行的，其它节点不执行该引脚的逻辑）
  ;  5.转换函数或事件的参数顺序必须一对一，例如：函数参数一必须对应转换节点参数一，函数参数二必须对应转换节点参数二
  ;  6.定义的函数请不要有返回值，如果实在需要返回值可以实现逻辑内结果保存到一个中间类，各个结点再去取
  ;  7.转换过后的函数或事件在非Ndisplay启动模式下也同样可以当普通函数执行，不受任何影响
  ;;[1 0 0.1829] 错误示范  Error demonstration
  (`KismetSystemLibrary.PrintString` "TODO") ; TODO
)

(event `TestEvent2`
  (params (Param1 :type Boolean) (Param2 :type Byte) (Param3 :type "Float (double-precision)"))
  ;[1 1 1] 用于多节点事件分发，只需要为其指定函数的参数，就可以在主节点上将事件分发并执行在各个结点上，注意这个节点必须被放置在自定义事件或者函数的第一个
  ; 支持函数和事件的转换，但尽量保证转换节点放置在第一个，否则转换节点前面的逻辑可能会被执行多次
  ; 注意：
  ;  1.可以使用普通函数或者事件去调用被转换后的函数或事件，且可以连续调用，但是不要短时间内调用同一个被转换后的函数或者事件（名字相同的）多次，否则可能只能执行一次
  ;  2.正在转换的函数或者事件内部请不要去调用其他已转换的事件或者函数，否则可能会导致执行顺序混乱且多次执行
  ;  3.转换事件尽量写在每个节点都会存在的对象上（因为转换节点需要通过该对象寻找函数，如果写在一个非各个结点都存在的对象上会导致那个节点无法执行目标函数）
  ;  4.尽量只用ExecuteMultiNodeEvent_Auto节点，如果非要使用ExecuteMultiNodeEvent那么每个节点需要执行的逻辑请写在NormalExe引脚，如果需要主机特例执行逻辑则写在MultiNodeExe（因为该引脚是主机分发事件执行前执行的，其它节点不执行该引脚的逻辑）
  ;  5.转换函数或事件的参数顺序必须一对一，例如：函数参数一必须对应转换节点参数一，函数参数二必须对应转换节点参数二
  ;  6.定义的函数请不要有返回值，如果实在需要返回值可以实现逻辑内结果保存到一个中间类，各个结点再去取
  ;  7.转换过后的函数或事件在非Ndisplay启动模式下也同样可以当普通函数执行，不受任何影响
  (`|TransformNDisFunc` Param1 Param2 Param3)
  (`KismetSystemLibrary.PrintString` (`KismetStringLibrary.Concat_StrStr` (`KismetStringLibrary.Conv_BoolToString` Param1) "---" (`KismetStringLibrary.Conv_ByteToString` Param2) "---" (`KismetStringLibrary.Conv_DoubleToString` Param3) "TODO")) ; TODO
)

(event `ERROR_TestEvent2`
  ;[1 1 1] 用于多节点事件分发，只需要为其指定函数的参数，就可以在主节点上将事件分发并执行在各个结点上，注意这个节点必须被放置在自定义事件或者函数的第一个
  ; 支持函数和事件的转换，但尽量保证转换节点放置在第一个，否则转换节点前面的逻辑可能会被执行多次
  ; 注意：
  ;  1.可以使用普通函数或者事件去调用被转换后的函数或事件，且可以连续调用，但是不要短时间内调用同一个被转换后的函数或者事件（名字相同的）多次，否则可能只能执行一次
  ;  2.正在转换的函数或者事件内部请不要去调用其他已转换的事件或者函数，否则可能会导致执行顺序混乱且多次执行
  ;  3.转换事件尽量写在每个节点都会存在的对象上（因为转换节点需要通过该对象寻找函数，如果写在一个非各个结点都存在的对象上会导致那个节点无法执行目标函数）
  ;  4.尽量只用ExecuteMultiNodeEvent_Auto节点，如果非要使用ExecuteMultiNodeEvent那么每个节点需要执行的逻辑请写在NormalExe引脚，如果需要主机特例执行逻辑则写在MultiNodeExe（因为该引脚是主机分发事件执行前执行的，其它节点不执行该引脚的逻辑）
  ;  5.转换函数或事件的参数顺序必须一对一，例如：函数参数一必须对应转换节点参数一，函数参数二必须对应转换节点参数二
  ;  6.定义的函数请不要有返回值，如果实在需要返回值可以实现逻辑内结果保存到一个中间类，各个结点再去取
  ;  7.转换过后的函数或事件在非Ndisplay启动模式下也同样可以当普通函数执行，不受任何影响
  ;;[1 0 0.1829] 错误示范  Error demonstration
  (`|TransformNDisFunc`)
  (`self.TestEvent1`))

(event `ERROR_TestEvent3`
  ;[1 1 1] 用于多节点事件分发，只需要为其指定函数的参数，就可以在主节点上将事件分发并执行在各个结点上，注意这个节点必须被放置在自定义事件或者函数的第一个
  ; 支持函数和事件的转换，但尽量保证转换节点放置在第一个，否则转换节点前面的逻辑可能会被执行多次
  ; 注意：
  ;  1.可以使用普通函数或者事件去调用被转换后的函数或事件，且可以连续调用，但是不要短时间内调用同一个被转换后的函数或者事件（名字相同的）多次，否则可能只能执行一次
  ;  2.正在转换的函数或者事件内部请不要去调用其他已转换的事件或者函数，否则可能会导致执行顺序混乱且多次执行
  ;  3.转换事件尽量写在每个节点都会存在的对象上（因为转换节点需要通过该对象寻找函数，如果写在一个非各个结点都存在的对象上会导致那个节点无法执行目标函数）
  ;  4.尽量只用ExecuteMultiNodeEvent_Auto节点，如果非要使用ExecuteMultiNodeEvent那么每个节点需要执行的逻辑请写在NormalExe引脚，如果需要主机特例执行逻辑则写在MultiNodeExe（因为该引脚是主机分发事件执行前执行的，其它节点不执行该引脚的逻辑）
  ;  5.转换函数或事件的参数顺序必须一对一，例如：函数参数一必须对应转换节点参数一，函数参数二必须对应转换节点参数二
  ;  6.定义的函数请不要有返回值，如果实在需要返回值可以实现逻辑内结果保存到一个中间类，各个结点再去取
  ;  7.转换过后的函数或事件在非Ndisplay启动模式下也同样可以当普通函数执行，不受任何影响
  ;;[1 0 0.1829] 错误示范  Error demonstration
  (`self.TestFunc1`))

(event `TestEvent3`
  (params (Param1 :type Boolean) (Param2 :type Byte) (NewParam :type Integer) (NewParam2 :type Integer64) (NewParam3 :type "Float (double-precision)") (NewParam4 :type "Vector Structure"))
  ;[1 1 1] 用于多节点事件分发，只需要为其指定函数的参数，就可以在主节点上将事件分发并执行在各个结点上，注意这个节点必须被放置在自定义事件或者函数的第一个
  ; 支持函数和事件的转换，但尽量保证转换节点放置在第一个，否则转换节点前面的逻辑可能会被执行多次
  ; 注意：
  ;  1.可以使用普通函数或者事件去调用被转换后的函数或事件，且可以连续调用，但是不要短时间内调用同一个被转换后的函数或者事件（名字相同的）多次，否则可能只能执行一次
  ;  2.正在转换的函数或者事件内部请不要去调用其他已转换的事件或者函数，否则可能会导致执行顺序混乱且多次执行
  ;  3.转换事件尽量写在每个节点都会存在的对象上（因为转换节点需要通过该对象寻找函数，如果写在一个非各个结点都存在的对象上会导致那个节点无法执行目标函数）
  ;  4.尽量只用ExecuteMultiNodeEvent_Auto节点，如果非要使用ExecuteMultiNodeEvent那么每个节点需要执行的逻辑请写在NormalExe引脚，如果需要主机特例执行逻辑则写在MultiNodeExe（因为该引脚是主机分发事件执行前执行的，其它节点不执行该引脚的逻辑）
  ;  5.转换函数或事件的参数顺序必须一对一，例如：函数参数一必须对应转换节点参数一，函数参数二必须对应转换节点参数二
  ;  6.定义的函数请不要有返回值，如果实在需要返回值可以实现逻辑内结果保存到一个中间类，各个结点再去取
  ;  7.转换过后的函数或事件在非Ndisplay启动模式下也同样可以当普通函数执行，不受任何影响
  ;;[1 1 1] 试用版本只支持bool uint8 int32 int64 float double Vector这七个类型,使用其它类型非完整版会导致崩溃
  (`|TransformNDisFunc` Param1 Param2 NewParam NewParam2 NewParam3 NewParam4)
  (`KismetSystemLibrary.PrintString` (`KismetStringLibrary.Concat_StrStr` (`KismetStringLibrary.Conv_BoolToString` Param1) "---" (`KismetStringLibrary.Conv_ByteToString` Param2) "---" (`KismetStringLibrary.Conv_IntToString` NewParam) "---" (`KismetStringLibrary.Conv_Int64ToString` NewParam2) "---" (`KismetStringLibrary.Conv_DoubleToString` NewParam3) (`KismetStringLibrary.Conv_VectorToString` NewParam4) "---" "TODO")) ; TODO
)

(event `self.ReceiveTick`
  (params (DeltaSeconds :type "Float (single-precision)"))
  ;[1 1 1] 用于多节点事件分发，只需要为其指定函数的参数，就可以在主节点上将事件分发并执行在各个结点上，注意这个节点必须被放置在自定义事件或者函数的第一个
  ; 支持函数和事件的转换，但尽量保证转换节点放置在第一个，否则转换节点前面的逻辑可能会被执行多次
  ; 注意：
  ;  1.可以使用普通函数或者事件去调用被转换后的函数或事件，且可以连续调用，但是不要短时间内调用同一个被转换后的函数或者事件（名字相同的）多次，否则可能只能执行一次
  ;  2.正在转换的函数或者事件内部请不要去调用其他已转换的事件或者函数，否则可能会导致执行顺序混乱且多次执行
  ;  3.转换事件尽量写在每个节点都会存在的对象上（因为转换节点需要通过该对象寻找函数，如果写在一个非各个结点都存在的对象上会导致那个节点无法执行目标函数）
  ;  4.尽量只用ExecuteMultiNodeEvent_Auto节点，如果非要使用ExecuteMultiNodeEvent那么每个节点需要执行的逻辑请写在NormalExe引脚，如果需要主机特例执行逻辑则写在MultiNodeExe（因为该引脚是主机分发事件执行前执行的，其它节点不执行该引脚的逻辑）
  ;  5.转换函数或事件的参数顺序必须一对一，例如：函数参数一必须对应转换节点参数一，函数参数二必须对应转换节点参数二
  ;  6.定义的函数请不要有返回值，如果实在需要返回值可以实现逻辑内结果保存到一个中间类，各个结点再去取
  ;  7.转换过后的函数或事件在非Ndisplay启动模式下也同样可以当普通函数执行，不受任何影响
  ;;[1 0 0.1829] 错误示范  Error demonstration
  ;;;[1 0 0.03535] 短时间内不要重复执行一个转换事件或函数
  ;;; Do not repeat a transformation event or function for a short period of time
  (`self.TestFunc1`))

(event `TestEvent5`
  (params (NewParam :type String) (NewParam2 :type "Float (double-precision)") (NewParam3 :type "Vector Structure") (NewParam4 :type "Actor Object Reference"))
  ;[1 1 1] 用于多节点事件分发，只需要为其指定函数的参数，就可以在主节点上将事件分发并执行在各个结点上，注意这个节点必须被放置在自定义事件或者函数的第一个
  ; 支持函数和事件的转换，但尽量保证转换节点放置在第一个，否则转换节点前面的逻辑可能会被执行多次
  ; 注意：
  ;  1.可以使用普通函数或者事件去调用被转换后的函数或事件，且可以连续调用，但是不要短时间内调用同一个被转换后的函数或者事件（名字相同的）多次，否则可能只能执行一次
  ;  2.正在转换的函数或者事件内部请不要去调用其他已转换的事件或者函数，否则可能会导致执行顺序混乱且多次执行
  ;  3.转换事件尽量写在每个节点都会存在的对象上（因为转换节点需要通过该对象寻找函数，如果写在一个非各个结点都存在的对象上会导致那个节点无法执行目标函数）
  ;  4.尽量只用ExecuteMultiNodeEvent_Auto节点，如果非要使用ExecuteMultiNodeEvent那么每个节点需要执行的逻辑请写在NormalExe引脚，如果需要主机特例执行逻辑则写在MultiNodeExe（因为该引脚是主机分发事件执行前执行的，其它节点不执行该引脚的逻辑）
  ;  5.转换函数或事件的参数顺序必须一对一，例如：函数参数一必须对应转换节点参数一，函数参数二必须对应转换节点参数二
  ;  6.定义的函数请不要有返回值，如果实在需要返回值可以实现逻辑内结果保存到一个中间类，各个结点再去取
  ;  7.转换过后的函数或事件在非Ndisplay启动模式下也同样可以当普通函数执行，不受任何影响
  (`BL_NDisplayEventSender.K2_TriggleMultiNodeEvent_Simple` (`|MakeArray` (`BL_NDisplayEventSender.InputParamToString` NewParam) (`BL_NDisplayEventSender.InputParamToString` NewParam2) (`BL_NDisplayEventSender.InputParamToString` NewParam3) (`BL_NDisplayEventSender.InputParamToString` NewParam4))
    (:`NormalExe`
      ;;[1 1 1] 这边的引脚将会执行在各个节点The pins on this side will be executed at each node
      (`KismetSystemLibrary.PrintString` "TODO"))
    (:`MultiNodeExe`
      ;;[1 1 1] 这边的引脚只有主节点会触发
      ;; The pins on this side only trigger the primary node
      (`KismetSystemLibrary.PrintString` "TODO"))))

(event `TestEvent4`
  (params (Param1 :type "Rotator Structure") (NewParam :type "Transform Structure") (NewParam2 :type "Actor Object Reference") (NewParam3 :type "ESplineMeshAxis Enum" :default "X") (NewParam4 :type "Anchors Structure") (NewParam5 :type "Array of Float (double-precision)"))
  (bind (_x _y) (`KismetMathLibrary.BreakVector2D` (`.Minimum` (break `Anchors` NewParam4))))
  ;[1 1 1] 用于多节点事件分发，只需要为其指定函数的参数，就可以在主节点上将事件分发并执行在各个结点上，注意这个节点必须被放置在自定义事件或者函数的第一个
  ; 支持函数和事件的转换，但尽量保证转换节点放置在第一个，否则转换节点前面的逻辑可能会被执行多次
  ; 注意：
  ;  1.可以使用普通函数或者事件去调用被转换后的函数或事件，且可以连续调用，但是不要短时间内调用同一个被转换后的函数或者事件（名字相同的）多次，否则可能只能执行一次
  ;  2.正在转换的函数或者事件内部请不要去调用其他已转换的事件或者函数，否则可能会导致执行顺序混乱且多次执行
  ;  3.转换事件尽量写在每个节点都会存在的对象上（因为转换节点需要通过该对象寻找函数，如果写在一个非各个结点都存在的对象上会导致那个节点无法执行目标函数）
  ;  4.尽量只用ExecuteMultiNodeEvent_Auto节点，如果非要使用ExecuteMultiNodeEvent那么每个节点需要执行的逻辑请写在NormalExe引脚，如果需要主机特例执行逻辑则写在MultiNodeExe（因为该引脚是主机分发事件执行前执行的，其它节点不执行该引脚的逻辑）
  ;  5.转换函数或事件的参数顺序必须一对一，例如：函数参数一必须对应转换节点参数一，函数参数二必须对应转换节点参数二
  ;  6.定义的函数请不要有返回值，如果实在需要返回值可以实现逻辑内结果保存到一个中间类，各个结点再去取
  ;  7.转换过后的函数或事件在非Ndisplay启动模式下也同样可以当普通函数执行，不受任何影响
  ;;[1 1 1] 完整版可以支持更多类型，包含对象，枚举，结构体，自定义结构体，数组，字典，列表等
  (`|TransformNDisFunc` Param1 NewParam NewParam2 NewParam3 NewParam4 NewParam5)
  ;;[1 1 1] TODO
  (`/Engine/EditorBlueprintResources/StandardMacros.IsValid` NewParam2
    (:`Is Valid`
      (`self.K2_SetActorRotation` NewParam2 Param1 false)
      (`self.K2_SetActorTransform` NewParam2 NewParam false false)
      (`KismetSystemLibrary.PrintString` (`|GetEnumeratorNameAsString` NewParam3))
      (`KismetSystemLibrary.PrintString` (`KismetStringLibrary.Concat_StrStr` (`KismetStringLibrary.Conv_DoubleToString` _x) "-" (`KismetStringLibrary.Conv_DoubleToString` _y)))
      (for _array_element NewParam5
        (`KismetSystemLibrary.PrintString` (`KismetStringLibrary.Conv_DoubleToString` _array_element))))))

(event `Call1`
  ;[0.005056 1 0] 调用 Call
  (`self.TestEvent1`))

(event `Call2`
  ;[0.005056 1 0] 调用 Call
  (`self.TestEvent1`)
  (`self.TestEvent2` true 1 234.0))

(fn `ERROR_TestFunc`
  (params (Param1 :type Boolean) (Param2 :type Byte) (Param3 :type "Float (double-precision)"))
  ;[1 1 1] 节点前面不要放置逻辑
  (`KismetSystemLibrary.PrintString` "Hello") ; TODO
)

(fn `TestFunc1`
  (`|TransformNDisFunc`)
  (`KismetSystemLibrary.PrintString` "TODO") ; TODO
)

(fn `TestFunc2`
  (params (Param1 :type Boolean) (Param2 :type Byte) (Param3 :type "Float (double-precision)"))
  (`|TransformNDisFunc` Param1 Param2 Param3)
  (`KismetSystemLibrary.PrintString` (`KismetStringLibrary.Concat_StrStr` (`KismetStringLibrary.Conv_BoolToString` Param1) "---" (`KismetStringLibrary.Conv_ByteToString` Param2) "---" (`KismetStringLibrary.Conv_DoubleToString` Param3) "TODO")) ; TODO
)

(fn `UserConstructionScript`)